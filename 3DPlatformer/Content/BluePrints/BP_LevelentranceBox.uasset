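; BP_LevelentranceBox is a level entrance trigger for the 3D platformer that loads another level when BP_ThirdPersonCharacter overlaps it.
; The LevelOpener index selects the level name from LevelList.
; On BeginPlay, it checks key flags in BP_3DPlatformerGameInstance and destroys itself if its matching key is set, removing that entrance.
; Only indices 2, 3 and 4 have key checks, mapped to Key2, Key1 and Key3 respectively.
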(event `self.ReceiveActorBeginOverlap`
  (params (OtherActor :type "Actor Object Reference"))
  (cast `/Game/ThirdPerson/Blueprints/BP_ThirdPersonCharacter` OtherActor)
  (`GameplayStatics.OpenLevel` (`KismetStringLibrary.Conv_StringToName` (`|GetArrayItem` (`self.LevelList`) (`self.LevelOpener`)))))

(event `self.ReceiveBeginPlay`
  (bind _asbp_3dplatformer_game_instance (cast `/Game/BP_3DPlatformerGameInstance` (`GameplayStatics.GetGameInstance`)))
  (set `self.As BP 3DPlatformer Game Instance` _asbp_3dplatformer_game_instance)
  (if (and (== (`self.LevelOpener`) 2) (`/Game/BP_3DPlatformerGameInstance.Key2` (`self.As BP 3DPlatformer Game Instance`)))
    (`self.K2_DestroyActor`)
    (elif (and (== (`self.LevelOpener`) 3) (`/Game/BP_3DPlatformerGameInstance.Key1` (`self.As BP 3DPlatformer Game Instance`)))
      (`self.K2_DestroyActor`)
      (elif (and (== (`self.LevelOpener`) 4) (`/Game/BP_3DPlatformerGameInstance.Key3` (`self.As BP 3DPlatformer Game Instance`)))
        (`self.K2_DestroyActor`)))))

(fn `UserConstructionScript`)