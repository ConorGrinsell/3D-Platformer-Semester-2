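; BP_Key is a collectible key pickup for a 3D platformer, configured by a KeyNumber selecting the living room, kitchen or bar room key.
; When the third-person character overlaps its Box, it sets the matching has-key flag on the character and the matching key flag in the game instance.
; The key then destroys itself once the game instance is updated, with debug prints only on the living room branch.
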(event `self.Box.OnComponentBeginOverlap`
  (params (OverlappedComponent :type "PrimitiveComponent Object Reference") (OtherActor :type "Actor Object Reference") (OtherComp :type "PrimitiveComponent Object Reference") (OtherBodyIndex :type Integer) (bFromSweep :type Boolean) (SweepResult :type "HitResult Structure (by ref)"))
  (bind _keynumber (`self.KeyNumber`))
  (bind _asbp_third_person_character (cast `/Game/ThirdPerson/Blueprints/BP_ThirdPersonCharacter` OtherActor))
  (if (== _keynumber 1)
    (set `/Game/ThirdPerson/Blueprints/BP_ThirdPersonCharacter.HasKey1(LivingRoom)` true _asbp_third_person_character)
    (bind _asbp_3dplatformer_game_instance (cast `/Game/BP_3DPlatformerGameInstance` (`GameplayStatics.GetGameInstance`))
      (:`then`
        (set `/Game/BP_3DPlatformerGameInstance.Key1` true _asbp_3dplatformer_game_instance)
        (`KismetSystemLibrary.PrintString` "collected")
        (`self.K2_DestroyActor`))
      (:`CastFailed`
        (`KismetSystemLibrary.PrintString` "Hello")))
    (elif (== _keynumber 2)
      (set `/Game/ThirdPerson/Blueprints/BP_ThirdPersonCharacter.HasKey2(Kitchen)` true _asbp_third_person_character)
      (bind _asbp_3dplatformer_game_instance_2 (cast `/Game/BP_3DPlatformerGameInstance` (`GameplayStatics.GetGameInstance`)))
      (set `/Game/BP_3DPlatformerGameInstance.Key2` true _asbp_3dplatformer_game_instance_2)
      (`self.K2_DestroyActor`)
      (elif (== _keynumber 3)
        (set `/Game/ThirdPerson/Blueprints/BP_ThirdPersonCharacter.HasKey3(BarRoom)` true _asbp_third_person_character)
        (bind _asbp_3dplatformer_game_instance_3 (cast `/Game/BP_3DPlatformerGameInstance` (`GameplayStatics.GetGameInstance`)))
        (set `/Game/BP_3DPlatformerGameInstance.Key3` true _asbp_3dplatformer_game_instance_3)
        (`self.K2_DestroyActor`)))))

(fn `UserConstructionScript`)