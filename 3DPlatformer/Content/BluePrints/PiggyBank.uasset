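; PiggyBank is a money pickup for a 3D platformer that adds one to the third-person character's Money on overlap.
; On BeginPlay it caches the game instance and starting location, then plays the Wiggle timeline to offset its height and set its yaw.
; When the character overlaps its Box, it copies the new total to MoneyGI on the game instance and destroys itself.
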(event `self.ReceiveBeginPlay`
  (bind (_returnvalue_x _returnvalue_y _returnvalue_z) (`KismetMathLibrary.BreakVector` (`self.K2_GetActorLocation`)))
  (bind _asbp_3dplatformer_game_instance (cast `/Game/BP_3DPlatformerGameInstance` (`GameplayStatics.GetGameInstance`)))
  (set `self.As BP 3DPlatformer Game Instance` _asbp_3dplatformer_game_instance)
  (set `self.Default Height` _returnvalue_z)
  (set `self.Return Value X` _returnvalue_x)
  (set `self.Return Value Y` _returnvalue_y)
  (bind (_direction _newtrack_0 _rotation) (`Timeline|Wiggle` :!via `PlayFromStart`)
    (:`Update`
      (`self.K2_SetActorLocationAndRotation` (`KismetMathLibrary.MakeVector` (`self.Return Value X`) (`self.Return Value Y`) (+ _newtrack_0 (`self.Default Height`))) (`KismetMathLibrary.MakeRotator` 0.0 0.0 _rotation)))))

(event `self.Box.OnComponentBeginOverlap`
  (params (OverlappedComponent :type "PrimitiveComponent Object Reference") (OtherActor :type "Actor Object Reference") (OtherComp :type "PrimitiveComponent Object Reference") (OtherBodyIndex :type Integer) (bFromSweep :type Boolean) (SweepResult :type "HitResult Structure (by ref)"))
  (bind _asbp_third_person_character (cast `/Game/ThirdPerson/Blueprints/BP_ThirdPersonCharacter` OtherActor))
  (bind _output_get (set `/Game/ThirdPerson/Blueprints/BP_ThirdPersonCharacter.Money` (+ (`/Game/ThirdPerson/Blueprints/BP_ThirdPersonCharacter.Money` _asbp_third_person_character) 1) _asbp_third_person_character))
  (set `/Game/BP_3DPlatformerGameInstance.Money(GI)` _output_get (`self.As BP 3DPlatformer Game Instance`))
  (`self.K2_DestroyActor`))

(fn `UserConstructionScript`)