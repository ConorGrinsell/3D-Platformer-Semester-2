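; Platform actor that endlessly cycles between disappearing and reappearing on a fixed timer.
; From BeginPlay, a looped chain of delays hides the cube and disables its collision, then restores both.
; A spotlight turns blue-violet when the platform appears and red shortly before it vanishes, signalling the coming change.
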(event `self.ReceiveBeginPlay`
  (bind _cube (`self.Cube`))
  (`PrimitiveComponent.SetCollisionEnabled` _cube "NoCollision" :!label _label)
  (`SceneComponent.SetVisibility` _cube false false)
  (`KismetSystemLibrary.Delay` 2.0)
  (`LightComponent.SetLightColor` (`self.SpotLight`) (struct :`R` 0.053159 :`B` 0.588542 :`A` 1.0) true)
  (`PrimitiveComponent.SetCollisionEnabled` _cube "QueryAndPhysics")
  (`SceneComponent.SetVisibility` _cube true false)
  (`KismetSystemLibrary.Delay` 1.2)
  (`LightComponent.SetLightColor` (`self.SpotLight`) (struct :`R` 0.395833 :`B` 0.006468 :`A` 1.0) true)
  (`KismetSystemLibrary.Delay` 0.8)
  (goto _label))

(fn `UserConstructionScript`)