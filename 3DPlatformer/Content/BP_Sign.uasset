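; BP_Sign is a sign actor that shows its text only while something overlaps its trigger box.
; On BeginPlay it copies SignText into a TextRender component and hides it.
; Box begin and end overlap events toggle the text's visibility and keep the TextVisible flag in sync, with no filter on the overlapping actor.
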(event `self.ReceiveBeginPlay`
  (bind _textrender (`self.TextRender`))
  (`TextRenderComponent.K2_SetText` _textrender (`self.SignText`))
  (`SceneComponent.SetVisibility` _textrender false false)
  (set `self.Text Visible?` false))

(event `self.Box.OnComponentBeginOverlap`
  (params (OverlappedComponent :type "PrimitiveComponent Object Reference") (OtherActor :type "Actor Object Reference") (OtherComp :type "PrimitiveComponent Object Reference") (OtherBodyIndex :type Integer) (bFromSweep :type Boolean) (SweepResult :type "HitResult Structure (by ref)"))
  (`SceneComponent.SetVisibility` (`self.TextRender`) true false)
  (set `self.Text Visible?` true))

(event `self.Box.OnComponentEndOverlap`
  (params (OverlappedComponent :type "PrimitiveComponent Object Reference") (OtherActor :type "Actor Object Reference") (OtherComp :type "PrimitiveComponent Object Reference") (OtherBodyIndex :type Integer))
  (`SceneComponent.SetVisibility` (`self.TextRender`) false false)
  (set `self.Text Visible?` false))

(fn `UserConstructionScript`)