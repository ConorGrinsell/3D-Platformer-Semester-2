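; BP_SwingingAxe is a swinging axe hazard that kills the third-person player character on contact.
; On BeginPlay it caches its roll and yaw, slows the AxeSwingRotation timeline, and starts it after a short random delay, so instances can start out of phase.
; The timeline drives the root component's pitch while keeping the cached roll and yaw.
; Overlapping either of two cube components calls DeathOperations on BP_ThirdPersonCharacter.
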(event `self.ReceiveBeginPlay`
  (bind (_returnvalue_roll _returnvalue_pitch _returnvalue_yaw) (`KismetMathLibrary.BreakRotator` (`self.K2_GetActorRotation`)))
  (set `self.Base Roll` _returnvalue_roll)
  (set `self.Base Yaw` _returnvalue_yaw)
  (`TimelineComponent.SetPlayRate` (`self.AxeSwingRotation`) 0.7)
  (`KismetSystemLibrary.Delay` (`KismetMathLibrary.RandomFloatInRange` 0.0 2.0))
  (bind (_direction _rotation) (`Timeline|AxeSwingRotation` :!via `PlayFromStart`)
    (:`Update`
      (`SceneComponent.K2_SetRelativeRotation` (`self.DefaultSceneRoot`) (`KismetMathLibrary.MakeRotator` (`self.Base Roll`) _rotation (`self.Base Yaw`)) false false))))

(event `self.Cube.OnComponentBeginOverlap`
  (params (OverlappedComponent :type "PrimitiveComponent Object Reference") (OtherActor :type "Actor Object Reference") (OtherComp :type "PrimitiveComponent Object Reference") (OtherBodyIndex :type Integer) (bFromSweep :type Boolean) (SweepResult :type "HitResult Structure (by ref)"))
  (bind _asbp_third_person_character (cast `/Game/ThirdPerson/Blueprints/BP_ThirdPersonCharacter` OtherActor))
  (`/Game/ThirdPerson/Blueprints/BP_ThirdPersonCharacter.Death Operations` _asbp_third_person_character))

(event `self.Cube1.OnComponentBeginOverlap`
  (params (OverlappedComponent :type "PrimitiveComponent Object Reference") (OtherActor :type "Actor Object Reference") (OtherComp :type "PrimitiveComponent Object Reference") (OtherBodyIndex :type Integer) (bFromSweep :type Boolean) (SweepResult :type "HitResult Structure (by ref)"))
  (bind _asbp_third_person_character (cast `/Game/ThirdPerson/Blueprints/BP_ThirdPersonCharacter` OtherActor))
  (`/Game/ThirdPerson/Blueprints/BP_ThirdPersonCharacter.Death Operations` _asbp_third_person_character))

(fn `UserConstructionScript`)