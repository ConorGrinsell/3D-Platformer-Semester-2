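; Test enemy that patrols using a timeline and kills the third-person character on Killbox overlap.
; The MovementRotation timeline offsets yaw from its starting value and adds movement along world X or Y, chosen by that starting yaw.
; GetStunned pauses movement, scales the Killbox to zero and plays a HitBounce height timeline, then restores both after a short delay.
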(event `self.ReceiveBeginPlay`
  (bind (_returnvalue_x _returnvalue_y _returnvalue_z) (`KismetMathLibrary.BreakVector` (`self.K2_GetActorLocation`)))
  (bind (_returnvalue_roll _returnvalue_pitch _returnvalue_yaw) (`KismetMathLibrary.BreakRotator` (`self.K2_GetActorRotation`)))
  (bind (_returnvalue_roll_2 _returnvalue_pitch_2) (`KismetMathLibrary.BreakRotator` (`self.K2_GetActorRotation`)))
  (bind _normal_rotation (`self.Normal Rotation`))
  (set `self.Normal Rotation` _returnvalue_yaw)
  (bind (_direction _movement _rotation) (`Timeline|Movement & Rotation` :!via `PlayFromStart` :!label _label)
    (:`Update`
      (set `self.Old X` _returnvalue_x)
      (set `self.Old Y` _returnvalue_y)
      (set `self.Old Z` _returnvalue_z)
      (set `self.Current Yaw` (+ _rotation (`self.Normal Rotation`)))
      (set `self.Current Roll` _returnvalue_roll_2)
      (set `self.Current Pitch` _returnvalue_pitch_2)
      (if (or (or (== 90.0 _normal_rotation) (== _normal_rotation 270.0)) (or (== _normal_rotation -90.0) (== _normal_rotation -270.0)))
        (`self.K2_SetActorTransform` (`KismetMathLibrary.MakeTransform` (`KismetMathLibrary.MakeVector` (`self.Old X`) (+ _movement _returnvalue_y) (`self.Old Z`)) (`KismetMathLibrary.MakeRotator` (`self.Current Roll`) (`self.Current Pitch`) (`self.Current Yaw`))))
        (else
          (`self.K2_SetActorTransform` (`KismetMathLibrary.MakeTransform` (`KismetMathLibrary.MakeVector` (+ _movement _returnvalue_x) (`self.Old Y`) (`self.Old Z`)) (`KismetMathLibrary.MakeRotator` (`self.Current Roll`) (`self.Current Pitch`) (`self.Current Yaw`)))))))))

(event `Get Stunned`
  (bind (_returnvalue_x _returnvalue_y _returnvalue_z) (`KismetMathLibrary.BreakVector` (`self.K2_GetActorLocation`)))
  (if (not (`self.Stunned`))
    (set `self.Stunned` true)
    (`SceneComponent.SetWorldScale3D` (`self.Killbox`) (0.0 0.0 0.0))
    (`|ExecutionSequence`
      (:`then_0`
        (goto _label :!via `Stop`))
      (:`then_1`
        (bind (_direction _height) (`Timeline|Hit Bounce` :!via `PlayFromStart`)
          (:`Update`
            (`self.K2_SetActorLocation` (`KismetMathLibrary.MakeVector` _returnvalue_x _returnvalue_y (+ _returnvalue_z _height))))
          (:`Finished`
            (`KismetSystemLibrary.Delay` 0.2)
            (set `self.Stunned` false)
            (`SceneComponent.SetWorldScale3D` (`self.Killbox`) (1.0 1.0 1.0))
            (goto _label)))))))

(event `self.Killbox.OnComponentBeginOverlap`
  (params (OverlappedComponent :type "PrimitiveComponent Object Reference") (OtherActor :type "Actor Object Reference") (OtherComp :type "PrimitiveComponent Object Reference") (OtherBodyIndex :type Integer) (bFromSweep :type Boolean) (SweepResult :type "HitResult Structure (by ref)"))
  (bind _asbp_third_person_character (cast `/Game/ThirdPerson/Blueprints/BP_ThirdPersonCharacter` OtherActor))
  (`/Game/ThirdPerson/Blueprints/BP_ThirdPersonCharacter.Death Operations` _asbp_third_person_character))

(fn `UserConstructionScript`)