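; BP_Enemy is a patrolling enemy that kills the third-person player character on contact with its Killbox.
; A MovementRotation timeline offsets its position along world X or Y, chosen from its starting yaw, and rotates it relative to that yaw.
; GetStunned pauses the patrol, shrinks the Killbox to zero scale and plays a HitBounce height timeline.
; After a short delay, it restores the Killbox and resumes movement.
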(event `self.ReceiveBeginPlay`
  (bind (_returnvalue_x _returnvalue_y _returnvalue_z) (`KismetMathLibrary.BreakVector` (`self.K2_GetActorLocation`)))
  (bind (_returnvalue_roll _returnvalue_pitch _returnvalue_yaw) (`KismetMathLibrary.BreakRotator` (`self.K2_GetActorRotation`)))
  (bind (_returnvalue_roll_2 _returnvalue_pitch_2) (`KismetMathLibrary.BreakRotator` (`self.K2_GetActorRotation`)))
  (bind _normal_rotation (`self.Normal Rotation`))
  (set `self.Normal Rotation` _returnvalue_yaw)
  (bind (_direction _movement _rotation) (`Timeline|Movement & Rotation` :!via `PlayFromStart` :!label _label)
    (:`Update`
      (if (or (or (== 90.0 _normal_rotation) (== _normal_rotation 270.0)) (or (== _normal_rotation -90.0) (== _normal_rotation -270.0)))
        (bind _returnvalue (+ _rotation (`self.Normal Rotation`)))
        (`self.K2_SetActorTransform` (`KismetMathLibrary.MakeTransform` (`KismetMathLibrary.MakeVector` _returnvalue_x (+ _returnvalue_y _movement) _returnvalue_z) (`KismetMathLibrary.MakeRotator` _returnvalue_roll_2 _returnvalue_pitch_2 _returnvalue)))
        (else
          (`self.K2_SetActorTransform` (`KismetMathLibrary.MakeTransform` (`KismetMathLibrary.MakeVector` (+ _movement _returnvalue_x) _returnvalue_y _returnvalue_z) (`KismetMathLibrary.MakeRotator` _returnvalue_roll_2 _returnvalue_pitch_2 _returnvalue))))))))

(event `Get Stunned`
  (bind (_returnvalue_x _returnvalue_y _returnvalue_z) (`KismetMathLibrary.BreakVector` (`self.K2_GetActorLocation`)))
  (if (not (`self.Stunned`))
    (set `self.Stunned` true)
    (`SceneComponent.SetWorldScale3D` (`self.Killbox`) (0.0 0.0 0.0))
    (`|ExecutionSequence`
      (:`then_0`
        (goto _label :!via `Stop`))
      (:`then_1`
        (bind (_direction _height) (`Timeline|Hit Bounce` :!via `PlayFromStart`)
          (:`Update`
            (`self.K2_SetActorLocation` (`KismetMathLibrary.MakeVector` _returnvalue_x _returnvalue_y (+ _height _returnvalue_z))))
          (:`Finished`
            (`KismetSystemLibrary.Delay` 0.2)
            (set `self.Stunned` false)
            (`SceneComponent.SetWorldScale3D` (`self.Killbox`) (1.0 1.0 1.0))
            (goto _label)))))))

(event `self.Killbox.OnComponentBeginOverlap`
  (params (OverlappedComponent :type "PrimitiveComponent Object Reference") (OtherActor :type "Actor Object Reference") (OtherComp :type "PrimitiveComponent Object Reference") (OtherBodyIndex :type Integer) (bFromSweep :type Boolean) (SweepResult :type "HitResult Structure (by ref)"))
  (bind _asbp_third_person_character (cast `/Game/ThirdPerson/Blueprints/BP_ThirdPersonCharacter` OtherActor))
  (`/Game/ThirdPerson/Blueprints/BP_ThirdPersonCharacter.Death Operations` _asbp_third_person_character))

(fn `UserConstructionScript`)