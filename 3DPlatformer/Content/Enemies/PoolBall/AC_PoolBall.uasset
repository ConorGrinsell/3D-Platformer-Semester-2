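; Actor component for a pool ball enemy that drifts its owner between random TargetPoints in the level.
; BeginPlay gathers every TargetPoint and picks one as the current target.
; Each Tick interpolates the owner toward it without sweep, re-rolling the interp speed every frame, and picks another random point once within a small tolerance.
; A second, delay-looped movement chain is left unconnected and never runs.
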(event `self.ReceiveBeginPlay`
  ; Find Random Point
  (bind _outactors (`GameplayStatics.GetAllActorsOfClass` "/Script/Engine.TargetPoint"))
  (bind _output_get (set `self.TravelPoints` _outactors))
  (bind _output_get_2 (set `self.Current Target` (`KismetArrayLibrary.Array_Random` _output_get) :!label _label)))

(event `self.ReceiveTick`
  (params (DeltaSeconds :type "Float (single-precision)"))
  (bind _returnvalue (`self.GetOwner`))
  (bind _returnvalue_2 (`Actor.K2_GetActorLocation` _returnvalue))
  ; Ball Shmoovement
  (bind _returnvalue_3 (`Actor.K2_GetActorLocation` (stale `self.ReceiveBeginPlay` _output_get_2)))
  (`Actor.K2_SetActorLocation` _returnvalue (`KismetMathLibrary.VInterpTo` _returnvalue_2 _returnvalue_3 DeltaSeconds (`KismetMathLibrary.RandomFloatInRange` 0.7 1.5)) false false)
  ; Find New Random Point
  (if (== _returnvalue_2 _returnvalue_3 :`ErrorTolerance` 10.0)
    (goto _label)))