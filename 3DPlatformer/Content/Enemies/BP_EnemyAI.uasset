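; Rat enemy AI that chases the player on sight and attempts a one-hit kill up close.
; PawnSensing triggers FollowPlayer, which re-arms the attack and runs AIMoveTo toward the player.
; On arrival it freezes player movement, faces them, plays the attack montage, then line-traces forward after a short delay.
; A capsule hit calls the player's DeathOperations, a miss restores player speed, and Die destroys the enemy.
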(event `self.ReceiveBeginPlay`
  (set `self.Default Rotation` (`self.K2_GetActorRotation`)))

(event `self.PawnSensing.OnSeePawn`
  (params (Pawn :type "Pawn Object Reference"))
  (if (not (`self.Dead`))
    (set `self.SeeingPlayer` true)
    (`self.FollowPlayer`)))

(event `FollowPlayer`
  (bind (_returnvalue_x _returnvalue_y _returnvalue_z) (`KismetMathLibrary.BreakVector` (`self.K2_GetActorLocation`)))
  (bind (_returnvalue_x_2 _returnvalue_y_2) (`KismetMathLibrary.BreakVector` (`self.GetActorForwardVector`)))
  (bind (_returnvalue_roll _returnvalue_pitch _returnvalue_yaw) (`KismetMathLibrary.BreakRotator` (`self.K2_GetActorRotation`)))
  (bind (_default_rotation_roll _default_rotation_pitch) (`KismetMathLibrary.BreakRotator` (`self.Default Rotation`)))
  (bind _returnvalue (- _returnvalue_z 15.0))
  (set `self.CanAttack` true)
  (if (`self.SeeingPlayer`)
    (if (not (`self.Dead`))
      (`|AIMoveTo` self (0.0 0.0 0.0) (`GameplayStatics.GetPlayerCharacter` 0) 65.0
        (:`OnSuccess`
          (if (`self.Dead`)
            _
            (elif (`self.SeeingPlayer`)
              (if (`self.CanAttack`)
                (set `self.CanAttack` false)
                (bind _asbp_third_person_character (cast `/Game/ThirdPerson/Blueprints/BP_ThirdPersonCharacter` (`GameplayStatics.GetPlayerCharacter` 0)))
                (set `CharacterMovementComponent.MaxWalkSpeed` 0.0 (`Character.CharacterMovement` _asbp_third_person_character))
                (`self.K2_SetActorRotation` (`KismetMathLibrary.FindLookAtRotation` (`self.K2_GetActorLocation`) (`self.K2_GetActorLocation` _asbp_third_person_character)))
                (`self.PlayAnimMontage` "/Game/Animations/AI/Rat/RatAttack_Anim_Montage.RatAttack_Anim_Montage")
                (`KismetSystemLibrary.Delay` 0.4)
                (if (not (`self.Dead`))
                  (bind _outhit (`KismetSystemLibrary.LineTraceSingle` :`Start` (`KismetMathLibrary.MakeVector` _returnvalue_x _returnvalue_y _returnvalue) :`End` (`KismetMathLibrary.MakeVector` (+ (* _returnvalue_x_2 100.0) _returnvalue_x) (+ (* _returnvalue_y_2 100.0) _returnvalue_y) _returnvalue) :`TraceChannel` "TraceTypeQuery1" :`DrawDebugType` "ForDuration"))
                  (if (== (`.HitComponent` (`GameplayStatics.BreakHitResult` _outhit)) (`Character.CapsuleComponent` _asbp_third_person_character))
                    (`/Game/ThirdPerson/Blueprints/BP_ThirdPersonCharacter.Death Operations` _asbp_third_person_character)
                    (else
                      (`self.K2_SetActorRotation` (`KismetMathLibrary.MakeRotator` _default_rotation_roll _default_rotation_pitch _returnvalue_yaw))
                      (set `CharacterMovementComponent.MaxWalkSpeed` 540.0 (`Character.CharacterMovement` _asbp_third_person_character)))))))))))))

(event `Die`
  (set `self.Dead` true)
  (`self.K2_DestroyActor`))

(fn `UserConstructionScript`)